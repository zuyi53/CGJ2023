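; BP_item_master is a base item actor for interactable pickups, with empty use, effect and interaction-handling hooks.
; InteractWithObject calls ServerInteract, which checks CanInteract, runs the server handler, then calls Multicastinteract for local handling.
; On overlap, it sends item class, icon and stack size through BPI_pickupitem to the other actor, skipping other items derived from itself.
; The pickup path bypasses the interaction check and leaves the item in the world.
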(event Custom|InteractWithObject
  (params (Player :type Character%20BP%20Object%20Reference))
  ;[1 1 1] interaction
  (CallFunction|ServerInteract Player))

(event Custom|ServerInteract
  (params (Player :type Character%20BP%20Object%20Reference))
  ;[1 1 1] interaction
  (bind _caninteract (CallFunction|CanInteract Player))
  (if _caninteract
    (CallFunction|HandleinteractionServer Player)
    (CallFunction|Multicastinteract Player)))

(event Custom|Multicastinteract
  (params (Player :type Character%20BP%20Object%20Reference))
  ;[1 1 1] interaction
  (CallFunction|Handleinteractionlocal Player))

(event Custom|UseItem)

(event Custom|effect)

(event EventBeginPlay)

(event Collision|EventActorBeginOverlap
  (params (OtherActor :type Actor%20Object%20Reference))
  ;[1 1 1] pickup item
  (if (Utilities|DoesObjectImplementInterface OtherActor "/Game/Asset/BPI_pickupitem.BPI_pickupitem_C")
    (if (not (Utilities|ClassIsChildOf (Utilities|GetClass OtherActor) "BP_item_master_C"))
      (Class|BPIPickupitem|Pickupitem(Message) OtherActor (Variables|Default|GetitemClass) (Variables|Default|Getitemicon) (Variables|Default|GetStackSize)))))

(event EventTick
  (params (DeltaSeconds :type Float%20%28single-precision%29)))

(fn ConstructionScript)

(fn CanInteract
  (params (player :type Character%20BP%20Object%20Reference))
  (return (Variables|Default|GetCan%20Interact_0)))

(fn Handleinteractionlocal
  (params (Player :type Character%20BP%20Object%20Reference)))

(fn HandleinteractionServer
  (params (Player :type Character%20BP%20Object%20Reference)))