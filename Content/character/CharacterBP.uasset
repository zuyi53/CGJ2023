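; Player character Blueprint that creates the in-game HUD and a submenu widget, and handles object interaction and per-character special skills.
; Interaction line-traces from the camera for BP_item_master actors, checks CanInteract, then repeats the check in ServerInteract before interacting.
; The special action, gated by ghost state and cooldown, calls SkillActive, which switches on CharacterID between custom movement, a block wall, an energy blast and floating.
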(event Custom|ServerInteract
  (params (object :type BP%20Item%20Master%20Object%20Reference))
  (bind _caninteract (Default|CanInteract object self))
  (if _caninteract
    (Default|InteractwithObject object self)))

(event Input|EnhancedActionEvents|EnhancedInputActionIA_interact
  (params (ActionValue :type Boolean) (ElapsedSeconds :type Float%20%28double-precision%29) (TriggeredSeconds :type Float%20%28double-precision%29) (InputAction :type Input%20Action%20Object%20Reference :default "/Game/IA/IA_interact.IA_interact"))
  ;[1 1 1] interaction
  (:Triggered
    (bind _asbp_item_master (Utilities|Casting|CastToBP_item_master (Variables|Default|GetObjectLoockingAt)))
    (Default|InteractwithObject _asbp_item_master)))

(event Input|EnhancedActionEvents|EnhancedInputActionIA_interact
  (params (ActionValue :type Boolean) (ElapsedSeconds :type Float%20%28double-precision%29) (TriggeredSeconds :type Float%20%28double-precision%29) (InputAction :type Input%20Action%20Object%20Reference :default "/Game/IA/IA_interact.IA_interact"))
  (bind _returnvalue (Game|GetPlayerCameraManager 0))
  (bind _transformcomponent (Variables|/Script/Engine.PlayerCameraManager|GetTransformComponent _returnvalue))
  ;[1 1 1] interaction
  (:Triggered
    (bind _outhit (Collision|LineTraceForObjects "0, 0, 0" (+ (Transformation|GetWorldLocation _transformcomponent) (* (Math|Vector|GetForwardVector _transformcomponent) (Variables|Default|Getdistanceforward))) (Utilities|Array|MakeArray "ObjectTypeQuery1" "ObjectTypeQuery2") false 0 "None"))
    (if true
      (bind _asbp_item_master (Utilities|Casting|CastToBP_item_master (.HitActor (Collision|BreakHitResult _outhit))))
      (bind _caninteract (Default|CanInteract _asbp_item_master self))
      (if _caninteract
        (CallFunction|ServerInteract _asbp_item_master))
      (else
        (Variables|Default|SetObjectLoockingAt 0)))))

(event Input|EnhancedActionEvents|EnhancedInputActionIA_specialAction
  (params (ActionValue :type Boolean) (ElapsedSeconds :type Float%20%28double-precision%29) (TriggeredSeconds :type Float%20%28double-precision%29) (InputAction :type Input%20Action%20Object%20Reference :default "/Game/IA/IA_specialAction.IA_specialAction"))
  (:Triggered
    (if (not (Variables|Default|GetisGhost))
      (if (== (Variables|Default|GetSkill_CD) 0)
        (CallFunction|SkillActive (Variables|Default|GetCharacter%20ID))))))

(event EventBeginPlay
  ;[1 1 1] menu
  (bind _returnvalue (UserInterface|CreateWidget "/Game/Widget/W_InGameHUD.W_InGameHUD_C"))
  (bind _output_get (Variables|Default|SetHUD _returnvalue))
  (UserInterface|Viewport|AddtoViewport _output_get 0)
  (Input|SetInputModeGameandUI (Game|GetPlayerController 0) 0 "DoNotLock" true false))

(event Collision|EventActorBeginOverlap
  (params (OtherActor :type Actor%20Object%20Reference))
  ;[1 1 1] menu
)

(event Input|KeyboardEvents|M
  (params (Key :type Key%20Structure))
  ;[1 1 1] menu
  (:Pressed
    (bind _returnvalue (UserInterface|CreateWidget "/Game/Widget/W_Submenu.W_Submenu_C"))
    (Variables|Default|SetSubmenu _returnvalue)))

(fn ConstructionScript)

(fn SkillActive
  (params (CharacterID :type Integer))
  (bind _charactermovement (Variables|Character|GetCharacterMovement))
  (bind _blockwall (Variables|Default|GetBlockWall))
  (switch int CharacterID
    (:0
      ;[1 1 1] TUCHO
      (Pawn|Components|CharacterMovement|SetMovementMode _charactermovement "MOVE_Custom" 0)
      (Utilities|Time|SetTimerbyEvent 0 15.0)
      (Pawn|Components|CharacterMovement|SetMovementMode _charactermovement "MOVE_None" 0))
    (:1
      ;[1 1 1] OUTCH 墙体生成
      (Default|SpawnActor _blockwall)
      (Utilities|Time|SetTimerbyEvent 0 15.0)
      (Actor|DestroyActor _blockwall))
    (:2
      ;[1 1 1] HOTUC 气功球发射
      (Game|SpawnActorfromClass "/Game/Asset/BP_EnergeBlast.BP_EnergeBlast_C" (Transformation|GetWorldTransform (Variables|Default|GetBlastSpawnPost)) "AlwaysSpawn" "MultiplyWithRoot" 0 0))
    (:3
      ;[1 1 1] CHOUT 无视减速
      (Variables|Default|SetisFloating true)
      (Utilities|Time|SetTimerbyEvent 0 15.0)
      (Variables|Default|SetisFloating false))))

(fn GetPickupitemData
  (return 0))