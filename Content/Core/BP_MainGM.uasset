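; BP_MainGM is the main game logic for a timed local-multiplayer ghost game, handling setup and win/lose screens.
; On BeginPlay it shows the HUD, creates three extra local players possessing BP_Player characters, and culls shuffled raw Pepsi pickups inside that loop.
; After a short delay TurnGhost makes a random player a ghost.
; The win widget appears when a fixed timer ends; CheckPlayerLose shows the lose widget when three players are ghosts.
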(event Custom|CheckPlayerLose
  (Utilities|Array|Clear (Variables|Default|Getghostlist))
  (for _array_element (Variables|Default|GetPlayerList)
    (if (Variables|/Game/Core/BP_Player.BP_Player_C|GetbIsGhost _array_element)
      (Utilities|Array|Add (Variables|Default|Getghostlist) (Variables|/Game/Core/BP_Player.BP_Player_C|GetbIsGhost _array_element))))
  (if (== (Utilities|Array|Length (Variables|Default|Getghostlist)) 3)
    (CallFunction|PlayerLose)))

(event Custom|PlayerWin
  (bind _returnvalue (UserInterface|CreateWidget "/Game/Widget/WB_Win.WB_Win_C"))
  (UserInterface|Viewport|AddtoViewport _returnvalue 0))

(event Custom|PlayerLose
  (bind _returnvalue (UserInterface|CreateWidget "/Game/Widget/WB_Lose.WB_Lose_C"))
  (UserInterface|Viewport|AddtoViewport _returnvalue 0))

(event EventBeginPlay
  (Utilities|FlowControl|Sequence
    (:then_0
      (bind _returnvalue (UserInterface|CreateWidget "/Game/Widget/W_InGameHUD.W_InGameHUD_C"))
      (UserInterface|Viewport|AddtoViewport _returnvalue 0)
      (Variables|/Script/Engine.PlayerController|SetbShowMouseCursor (Game|GetPlayerController 0) true))
    (:then_1
      (Utilities|FlowControl|Sequence
        (:then_0
          (for _index (range 1 3)
            (bind _returnvalue_2 (Class|GameplayStatics|CreatePlayer _index))
            (bind _asbp_player (Utilities|Casting|CastToBP_Player (Game|GetPlayerCharacter _index)))
            (Default|SwitchImage _asbp_player _index)
            (Utilities|IsValid _returnvalue_2
              (:Is%20Valid
                (Pawn|Possess _returnvalue_2 _asbp_player)
                ;[1 1 1] 道具生成
                (bind _outactors (Actor|GetAllActorsOfClass "/Game/Asset/BP_item_rawPepsi.BP_item_rawPepsi_C"))
                (Utilities|Array|Shuffle _outactors)
                (Variables|Default|SetTotalCollectables (Utilities|Array|Length _outactors))
                (for _index_2 (range 0 (- (Utilities|Array|Length _outactors) (+ (Variables|Default|GetCollectablesInmap) 1)))
                  (Actor|DestroyActor (Utilities|Array|Get(acopy) _outactors _index_2))
                  (bind _output_get (Variables|Default|SetTotalCollectables (- (Variables|Default|GetTotalCollectables) 1)))
                  (Variables|Default|SetCollectablesInmap _output_get))))))
        (:then_1
          (Utilities|FlowControl|Delay 2e+01)
          (CallFunction|PlayerWin))
        (:then_2
          (Utilities|FlowControl|Delay 2.0)
          (CallFunction|TurnGhost))))))

(fn ConstructionScript)

(fn TurnGhost
  (bind _outactors (Actor|GetAllActorsOfClass "/Game/Core/BP_Player.BP_Player_C"))
  (Variables|Default|SetPlayerList _outactors)
  (Default|GhostMode (Utilities|Array|Get(acopy) (Variables|Default|GetPlayerList) (Math|Random|RandomIntegerinRange 0 3))))