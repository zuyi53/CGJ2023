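; Dynamic music controller that drives the FMOD music's danger intensity from how close players are to the main ghost.
; Every tick it finds the nearest non-ghost player's distance and maps it piecewise across Range thresholds to a 0–2 DangerLevel parameter on the current theme.
; TrunGhostTheme fades out the music bus and starts the indexed player's theme, guarded by a DoOnce.
; GhostSound plays a 2D ghost-pass stinger.
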(event Custom|TrunGhostTheme
  (params (player%20index :type Integer))
  ;[1 1 1] Comment
  (Utilities|FlowControl|DoOnce false
    (:Completed
      (Class|FMODBlueprintStatics|BusStopAllEvents "/Game/FMOD/Buses/Music.Music" "ALLOWFADEOUT")
      (bind _returnvalue (Class|FMODBlueprintStatics|PlayEvent2D (Utilities|Array|Get(acopy) (Variables|Default|GetPlayerThemeMusic) player%20index)))
      (Variables|Default|Setcurrent%20theme _returnvalue))))

(event Custom|GhostSound
  (Class|FMODBlueprintStatics|PlayEvent2D "/Game/FMOD/Events/Stingers/GhostPassStinger.GhostPassStinger"))

(event Custom|DynamicDanagerLvl
  (bind _range (Variables|Default|GetRange))
  (bind _range_2 (Variables|Default|GetRange))
  (bind _length (Variables|Default|Getlength))
  (bind _minvalue (Math|Float|MinOfFloatArray _length))
  (bind _output (Utilities|Array|Get(acopy) _range))
  (bind _output_2 (Utilities|Array|Get(acopy) _range_2 1))
  (Utilities|Array|Clear (Variables|Default|Getlength))
  (for _array_element (Variables|Default|GetPlayer)
    (if (not (Variables|/Game/Core/BP_Player.BP_Player_C|GetbIsGhost _array_element))
      (Utilities|Array|Add (Variables|Default|Getlength) (Math|Float|Absolute(Float) (Math|Vector|VectorLength (- (Transformation|GetActorLocation _array_element) (Transformation|GetActorLocation (Variables|Default|GetMainGhost))))))))
  (Variables|Default|Setval _minvalue)
  (if (> (Variables|Default|Getval) 1e+03)
    (Variables|Default|SetdanagerLevel 0.0)
    (Class|FMODBlueprintStatics|EventInstanceSetParameter (Variables|Default|Getcurrent%20theme) "DangerLevel" 0.0)
    (elif (and (< _minvalue (Utilities|Array|Get(acopy) (Variables|Default|GetRange))) (> _minvalue (Utilities|Array|Get(acopy) (Variables|Default|GetRange) 1)))
      (bind _output_get (Variables|Default|SetdanagerLevel (Math|Float|Absolute(Float) (/ (- (Variables|Default|Getval) _output) (- _output (Utilities|Array|Get(acopy) (Variables|Default|GetRange) 1))))))
      (Class|FMODBlueprintStatics|EventInstanceSetParameter (Variables|Default|Getcurrent%20theme) "DangerLevel" _output_get)
      (elif (and (< (Variables|Default|Getval) (Utilities|Array|Get(acopy) (Variables|Default|GetRange) 1)) (> (Variables|Default|Getval) (Utilities|Array|Get(acopy) (Variables|Default|GetRange) 2)))
        (bind _output_get_2 (Variables|Default|SetdanagerLevel (+ (Math|Float|Absolute(Float) (/ (- (Variables|Default|Getval) _output_2) (- _output_2 (Utilities|Array|Get(acopy) (Variables|Default|GetRange) 2)))) 1.0)))
        (Class|FMODBlueprintStatics|EventInstanceSetParameter (Variables|Default|Getcurrent%20theme) "DangerLevel" _output_get_2)
        (else
          (bind _output_get_3 (Variables|Default|SetdanagerLevel 2.0))
          (Class|FMODBlueprintStatics|EventInstanceSetParameter (Variables|Default|Getcurrent%20theme) "DangerLevel" _output_get_3))))))

(event EventTick
  (params (DeltaSeconds :type Float%20%28single-precision%29))
  ;[1 1 1] Comment
  (CallFunction|DynamicDanagerLvl))

(fn ConstructionScript)